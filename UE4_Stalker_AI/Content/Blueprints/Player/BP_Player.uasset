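; First-person player Blueprint that adds animation, camera and noise feedback to jump, weapon and damage events.
; Firing and reloading play rifle montages on the Arms mesh, while firing and taking point damage also trigger world camera shakes at the player's location.
; Jumping and firing call MakeNoise with the player as instigator, with gunfire carrying farther than jumps.
; It contains no shooting, ammo or health logic, only these cosmetic and noise responses.
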(event `self.OnJumped`
  (`self.MakeNoise` 1.0 self (`self.K2_GetActorLocation`) 5000.0))

(event `self.BP_OnFireWithWeapon`
  (bind _returnvalue (`self.K2_GetActorLocation`))
  (`|PlayMontage` (`self.Arms`) "/Game/Animations/FPP_Animations/HerroFPP_RifleFire_Montage.HerroFPP_RifleFire_Montage"
    (:`then`
      (`GameplayStatics.PlayWorldCameraShake` "/Game/Blueprints/CameraShakes/CameraShake_FireWithWeapon.CameraShake_FireWithWeapon_C" _returnvalue 0.0 400.0)
      (`self.MakeNoise` 1.0 self _returnvalue 10000.0))))

(event `self.BP_OnReloadWeapon`
  (`|PlayMontage` (`self.Arms`) "/Game/Animations/FPP_Animations/HeroFPP_RifleReload_Montage.HeroFPP_RifleReload_Montage"))

(event `self.ReceivePointDamage`
  (params (Damage :type "Float (single-precision)") (DamageType :type "DamageType Object Reference") (HitLocation :type "Vector Structure") (HitNormal :type "Vector Structure") (HitComponent :type "PrimitiveComponent Object Reference") (BoneName :type Name) (ShotFromDirection :type "Vector Structure") (InstigatedBy :type "Controller Object Reference") (DamageCauser :type "Actor Object Reference") (HitInfo :type "HitResult Structure (by ref)"))
  (`GameplayStatics.PlayWorldCameraShake` "/Game/Blueprints/CameraShakes/CameraShake_Damaged.CameraShake_Damaged_C" (`self.K2_GetActorLocation`) 0.0 400.0))

(fn `UserConstructionScript`)