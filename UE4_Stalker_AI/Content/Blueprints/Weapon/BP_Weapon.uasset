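; Weapon Blueprint that plays a randomized gunshot sound each time a bullet is fired.
; OnFiredBullet picks a random entry from FireSoundList and checks whether the owning pawn is player-controlled.
; Player-controlled weapons play the sound in 2D, while all others play it spatially at the weapon's location.
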(event `self.BP_OnFiredBullet`
  (params (HitLocation :type "Vector Structure (by ref)") (HitActor :type "Actor Object Reference"))
  (bind _newparam (`self.GetRandomFireSound`))
  (if (`self.IsPlayerControlled`)
    (`GameplayStatics.PlaySound2D` _newparam 1.0 1.0 0.0 null null)
    (else
      (`GameplayStatics.SpawnSoundAtLocation` _newparam (`self.K2_GetActorLocation`) (struct) 1.0 1.0 0.0 null null))))

(fn `GetRandomFireSound`
  (returns (NewParam :type "SoundWave Object Reference"))
  (bind _firesoundlist (`self.FireSoundList`))
  (return (`|GetArrayItem` _firesoundlist (`KismetMathLibrary.RandomIntegerInRange` 0 (- (`KismetArrayLibrary.Array_Length` _firesoundlist) 1)))))

(fn `IsPlayerControlled`
  (returns (IsPlayerController :type Boolean))
  (bind _aspawn (cast `Pawn` (`self.GetOwner`))
    (:`then`
      (return (`Pawn.IsPlayerControlled` _aspawn)))
    (:`CastFailed`
      (return false))))

(fn `UserConstructionScript`)